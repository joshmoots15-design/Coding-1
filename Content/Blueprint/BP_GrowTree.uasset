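; BP_GrowTree is an actor whose Cedar component grows when the third-person character overlaps it carrying water.
; On overlap it checks the character's TotalWaterCount and either runs the shared Grow logic or prints a prompt to get water.
; Growing adds a random amount to the tree's relative scale and prints a message, without reducing the water count.
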(event Custom|Grow
  (bind _cedar (Variables|Default|GetCedar))
  (Transformation|SetRelativeScale3D _cedar (+ (Variables|/Script/Engine.SceneComponent|GetRelativeScale3D _cedar) (Math|Random|RandomFloatinRange 0.2 1.0)))
  (Development|PrintText "Feed Me More!!!"))

(event Collision|EventActorBeginOverlap
  (params (OtherActor :type Actor%20Object%20Reference))
  (bind _cedar (Variables|Default|GetCedar))
  (bind _asbp_third_person_character (Utilities|Casting|CastToBP_ThirdPersonCharacter OtherActor))
  (if (> (Variables|/Game/ThirdPerson/Blueprints/BP_ThirdPersonCharacter.BP_ThirdPersonCharacter_C|GetTotalWaterCount _asbp_third_person_character) 0)
    (Transformation|SetRelativeScale3D _cedar (+ (Variables|/Script/Engine.SceneComponent|GetRelativeScale3D _cedar) (Math|Random|RandomFloatinRange 0.2 1.0)))
    (Development|PrintText "Feed Me More!!!")
    (else
      (Development|PrintText "Get Water"))))

(event EventTick
  (params (DeltaSeconds :type Float%20%28single-precision%29)))

(fn ConstructionScript)