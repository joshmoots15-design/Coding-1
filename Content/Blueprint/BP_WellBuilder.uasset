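; BP_WellBuilder is a pickup item that lets the third-person character place a water well.
; On overlap it stores the character and calls its TryToPickupItem, and the Pickup event attaches the item to the character's right-hand socket.
; PrimaryAction spawns a BP_WaterWell at the item's transform, while Drop destroys the item.
; Each action also prints a debug message.
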(event Collision|EventActorBeginOverlap
  (params (OtherActor :type Actor%20Object%20Reference))
  (bind _asbp_third_person_character (Utilities|Casting|CastToBP_ThirdPersonCharacter OtherActor))
  (Variables|Default|SetPlayrt _asbp_third_person_character)
  (Default|TrytoPickupItem _asbp_third_person_character self))

(event EventPickup
  (Development|PrintText "I got picked up")
  (Transformation|AttachComponentToComponent (Variables|/Script/Engine.Character|GetMesh (Variables|Default|GetPlayrt)) "HandGrip_R" "SnapToTarget" "SnapToTarget" "KeepRelative" true))

(event EventPrimaryAction
  (Development|PrintText "plant a rock")
  (Game|SpawnActorfromClass "/Game/Blueprint/BP_WaterWell.BP_WaterWell_C" (Transformation|GetActorTransform) "Undefined" "MultiplyWithRoot" 0 0))

(event EventDrop
  (Development|PrintText "Dropped It")
  (Actor|DestroyActor))

(fn ConstructionScript)