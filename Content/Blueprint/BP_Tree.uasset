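; Tree actor that grows in random steps after play begins.
; BeginPlay runs a delayed loop through a DoN gate, waiting a few random seconds before each Grow call.
; Grow adds a random uniform amount to the BPTree component's relative scale.
; The DoN limit is a pure random integer, re-rolled on each pass, so growth stops after at most five steps.
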(event Custom|Grow
  (bind _bp_tree (Variables|Default|GetBP_Tree))
  (Transformation|SetRelativeScale3D _bp_tree (+ (Variables|/Script/Engine.SceneComponent|GetRelativeScale3D _bp_tree) (Math|Random|RandomFloatinRange 0.2 0.6))))

(event EventBeginPlay
  (Utilities|FlowControl|DoN (Math|Random|RandomIntegerinRange 1 5) :!label _label
    (:Exit
      (Utilities|FlowControl|Delay (Math|Random|RandomFloatinRange 3.0 5.0))
      (CallFunction|Grow)
      (goto _label))))

(event Collision|EventActorBeginOverlap
  (params (OtherActor :type Actor%20Object%20Reference)))

(event EventTick
  (params (DeltaSeconds :type Float%20%28single-precision%29)))

(fn ConstructionScript)